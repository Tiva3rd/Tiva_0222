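; Actor component for resource gathering that rolls a chance to run a timing minigame granting a tiered reward multiplier.
; The server starts the game and timeout; InstigatorPawn's OnRep locks local input and opens the widget, while other clients spawn an overhead indicator.
; A looping timer ping-pongs the progress bar.
; Click or timeout triggers server cleanup, making the owner score proximity to the target, broadcast the result and restore input.
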(event Custom|InteruptGame)

(event EventBeginPlay
  ;[0 0 0] Begin Play
  (Networking|SwitchHasAuthority
    (:Authority
      (CallFunction|RandomStartingPointEveryGame? (Variables|DesiredPoint|GetRandomPointEveryGame?) 7e+01))))

(event EventTick
  (params (DeltaSeconds :type Float%20%28single-precision%29)))

(fn SpawnIndicatorWidget
  (bind _instigator_pawn (Variables|References|GetInstigator%20Pawn))
  (bind _returnvalue (Transformation|GetActorTransform _instigator_pawn))
  (bind _returnvalue_2 (Game|SpawnActorfromClass "/Game/GatheringResourcesSystem/Blueprints/BonusGameIndicator/BP_BonusGameIndicator.BP_BonusGameIndicator_C" (Math|Transform|MakeTransform (Math|Vector|MakeVector (.x (.location _returnvalue)) (.y (.location _returnvalue)) (+ (.z (.location _returnvalue)) (Variables|WidgetIndicator|GetIndicatorWidgetHeight))) "0, 0, 0" "1.000000,1.000000,1.000000") "AlwaysSpawn" 0 (Variables|WidgetIndicator|GetWidgetIndicatorClass) _instigator_pawn))
  (Variables|Utility|SetBonusGameIndicator _returnvalue_2)
  (return))

(fn CreateGameWidget
  (bind _returnvalue (UserInterface|CreateWidget "/Game/GatheringResourcesSystem/UI/Widgets/WBP_ResourceBonusGame.WBP_ResourceBonusGame_C" (.AsPlayer%20Controller (Utilities|Casting|CastToPlayerController (Variables|References|GetInstigator%20Controller))) (Variables|DesiredPoint|GetDesiredStopValue) self))
  (Variables|References|SetBonusGameWidget _returnvalue)
  (UserInterface|Viewport|AddtoViewport _returnvalue 0)
  (return))

(fn RandomStartingPointEveryGame?
  (params (useRandomStartingPoint? :type Boolean) (DesiredStop :type Float%20%28double-precision%29))
  (if useRandomStartingPoint?
    (Variables|DesiredPoint|SetDesiredStopValue (Math|Random|RandomFloatinRange 0.0 1e+02))
    (return)
    (else
      (Variables|DesiredPoint|SetDesiredStopValue DesiredStop))))

(fn LuckyRoll
  (return (< (Math|Random|RandomFloatinRange 0.0 1e+02) (Variables|BonusGame|GetChanceForBonusGame))))

(fn InterpPlayerHitValue
  (bind _desiredstopvalue (Variables|DesiredPoint|GetDesiredStopValue))
  (LocalVariables|SetMAX (+ _desiredstopvalue 4.0))
  (LocalVariables|SetMIN (- _desiredstopvalue 4.0))
  (if (Math|Float|InRange(Float) (Variables|Utility|GetPlayerHitValue) (LocalVariables|GetMIN) (LocalVariables|GetMAX))
    (return 0)
    (else
      (bind _index (Utilities|FlowControl|ForLoopwithBreak 1 3 :!label _label)
        (:LoopBody
          (bind _output_get (LocalVariables|SetIndexThatWon _index))
          (LocalVariables|SetMAX (+ (* _output_get (Variables|BonusGameValues|GetSteps)) (LocalVariables|GetMAX)))
          (LocalVariables|SetMIN (- (LocalVariables|GetMIN) (Math|Conversions|ToFloat(Integer) (* _output_get (Variables|BonusGameValues|GetSteps)))))
          (if (Math|Float|InRange(Float) (Variables|Utility|GetPlayerHitValue) (LocalVariables|GetMIN) (LocalVariables|GetMAX))
            (goto _label Break)))
        (:Completed
          (return (LocalVariables|GetIndexThatWon)))))))

(fn SetRewardBasedOfLevelHit
  (params (Index :type Integer))
  (return (Utilities|Select :Index Index :Option%200 (Variables|BonusGameValues|GetRewardLevel_4) :Option%201 (Variables|BonusGameValues|GetRewardLevel_3) :Option%202 (Variables|BonusGameValues|GetRewardLevel_2) :Option%203 (Variables|BonusGameValues|GetRewardLevel_1)) (Utilities|Select :Index Index :Option%200 "NewEnumerator0" :Option%201 "NewEnumerator1" :Option%202 "NewEnumerator2" :Option%203 "NewEnumerator3")))

(fn OnRepIsBonusGameRuning?
  (if (Pawn|IsLocallyControlled (Variables|References|GetInstigator%20Pawn))
    (CallFunction|StartBonusGame)
    (return)))

(fn IsGameAllowedtoPlay?
  (return (and (Variables|BonusGame|GetTurnGameON/OFF) (not (Variables|BonusGame|GetisBonusGameRuning?)))))

(fn StartBonusGame
  (bind _returnvalue (Utilities|Time|SetTimerbyFunctionName 0 "StartProgressBar" 0.01 true))
  (Variables|Utility|SetStartBonusGameTimerHandler _returnvalue))

(fn StartProgressBar
  (switch name (Variables|Utility|GetProgressBarDirectionIndicator)
    (:Add
      (bind _output_get (Variables|Utility|SetProgressBarValue (+ (Variables|Utility|GetProgressBarValue) (* (Class|KismetSystemLibrary|GetTimerElapsedTimeHandle (Variables|Utility|GetStartBonusGameTimerHandler)) (Variables|BonusGame|GetGameSpeed)))))
      (if (>= _output_get 1.0)
        (Variables|Utility|SetProgressBarDirectionIndicator "Negate")))
    (:Negate
      (bind _output_get_2 (Variables|Utility|SetProgressBarValue (- (Variables|Utility|GetProgressBarValue) (* (Class|KismetSystemLibrary|GetTimerElapsedTimeHandle (Variables|Utility|GetStartBonusGameTimerHandler)) (Variables|BonusGame|GetGameSpeed)))))
      (if (<= _output_get_2 0.0)
        (Variables|Utility|SetProgressBarDirectionIndicator "Add")))))

(fn GetProgressBarValue
  (return (Variables|Utility|GetProgressBarValue)))

(fn SetPlayerMode
  (params (InGame? :type Boolean))
  (bind _instigator_controller (Variables|References|GetInstigator%20Controller))
  (bind _instigator_controller_2 (Variables|References|GetInstigator%20Controller))
  (bind _instigator_pawn (Variables|References|GetInstigator%20Pawn))
  (bind _asplayer_controller (Utilities|Casting|CastToPlayerController _instigator_controller))
  (bind _asplayer_controller_2 (Utilities|Casting|CastToPlayerController _instigator_controller_2))
  (if InGame?
    (Components|Movement|StopMovementImmediately (Actor|GetComponentbyClass _instigator_pawn "/Script/Engine.CharacterMovementComponent"))
    (Input|DisableInput _instigator_pawn _asplayer_controller_2)
    (AI|Navigation|StopMovement _instigator_controller_2)
    (Input|SetInputModeUIOnly _asplayer_controller_2 (Variables|References|GetBonusGameWidget) "DoNotLock")
    (return)
    (else
      (Input|SetInputModeGameOnly _asplayer_controller)
      (Input|EnableInput (Variables|References|GetInstigator%20Pawn) _asplayer_controller)
      (return))))

(fn StopGame
  (Utilities|Time|ClearandInvalidateTimerbyHandle (Variables|Utility|GetStartBonusGameTimerHandler))
  (Variables|Utility|SetPlayerHitValue (* (Variables|Utility|GetProgressBarValue) 1e+02))
  (bind _reward (CallFunction|InterpPlayerHitValue))
  (bind (_multiplicationreward _rewardlevel) (CallFunction|SetRewardBasedOfLevelHit _reward))
  (Default|CallBonusGameRes _multiplicationreward _rewardlevel)
  (if (Pawn|IsLocalPlayerController (Variables|References|GetInstigator%20Controller))
    (CallFunction|SetPlayerMode false)
    (return)))

(fn OnRepInstigatorPawn
  (if (Pawn|IsLocallyControlled (Variables|References|GetInstigator%20Pawn))
    (CallFunction|SetPlayerMode true)
    (CallFunction|CreateGameWidget)
    (CallFunction|StartBonusGame)
    (return)
    (else
      (CallFunction|SpawnIndicatorWidget)
      (return))))

(fn StartGameTimer
  (bind _returnvalue (Utilities|Time|SetTimerbyFunctionName 0 "GameTimer" 1.0 true))
  (Variables|Utility|SetGameTimerHandler _returnvalue)
  (return))

(fn GameTimer
  (Math|Integer|IncrementInt (Variables|Utility|GetGameTime)
    (:%20%20
      (if (== (Variables|Utility|GetGameTime) (Variables|Utility|GetGameTimeMaximum%28Seconds%29))
        (CallFunction|ServerCleanUpGame)))))

(fn GetIsBonusGameRunning?
  (return (Variables|BonusGame|GetisBonusGameRuning?)))

(event Custom|TryStartBonusGame
  (params (Instigator%20Pawn :type Pawn%20Object%20Reference) (Instigator%20Controller :type Controller%20Object%20Reference))
  ;[0 0 0] SERVER
  (if (CallFunction|IsGameAllowedtoPlay?)
    (if (CallFunction|LuckyRoll)
      (Variables|BonusGame|SetisBonusGameRuning? true)
      (Actor|SetOwner (Components|GetOwner) Instigator%20Pawn)
      (Variables|References|SetInstigator%20Controller Instigator%20Controller)
      (Variables|References|SetInstigator%20Pawn Instigator%20Pawn)
      (CallFunction|StartGameTimer))))

(event Custom|Owning_StopGame
  ;[0 0 0] Called from the W_ResourceBonusGame once clicked to set the Hit value
  (CallFunction|StopGame))

(event Custom|Server_CleanUpGame
  ;[0 0 0] Called from the W_ResourceBonusGame once clicked to set the Hit value
  (Utilities|FlowControl|DoOnce false
    (:Completed
      (CallFunction|OwningStopGame)
      (CallFunction|MultiDestroyBonusGameIndicator)
      (Utilities|Time|ClearandInvalidateTimerbyHandle (Variables|Utility|GetGameTimerHandler)))))

(event Custom|Multi_DestroyBonusGameIndicator
  ;[0 0 0] Called from the W_ResourceBonusGame once clicked to set the Hit value
  (if (not (Pawn|IsLocallyControlled (Variables|References|GetInstigator%20Pawn)))
    (Default|OnDestroy (Variables|Utility|GetBonusGameIndicator))))