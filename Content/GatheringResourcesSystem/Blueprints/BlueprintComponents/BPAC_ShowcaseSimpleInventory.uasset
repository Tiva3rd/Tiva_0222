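; Actor component that provides a simple showcase inventory for the gathering resources system, storing items directly in UI slot widgets.
; InitializeInventory creates WBP_Inventory inside a given overlay and caches its slot array.
; Owning_TryAddItem merges quantity into a slot with matching name and tier, otherwise fills the first empty slot, then refreshes that slot.
; When no slot is free, it prints a message saying the inventory is full.
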(event Custom|Owning_TryAddItem
  (params (Item%20to%20Add :type S%20Item%20Structure))
  (bind _output_get (Variables|Default|SetItem%20to%20Add Item%20to%20Add))
  (bind _founditeminslot (Private|FindifThereIsSameItem _output_get))
  (Utilities|IsValid _founditeminslot
    (:Is%20Valid
      (Private|ShowIteminInventorySlot (Utilities|Struct|MakeS_Item (.Name (Utilities|Struct|BreakS_Item (Variables|Default|GetItem%20to%20Add))) (.Tier (Utilities|Struct|BreakS_Item (Variables|Default|GetItem%20to%20Add))) (+ (.Quantity (Utilities|Struct|BreakS_Item (Variables|Default|GetItem%20to%20Add))) (.Quantity (Utilities|Struct|BreakS_Item (Variables|/Game/GatheringResourcesSystem/UI/Widgets/WBP_InventorySlot.WBP_InventorySlot_C|GetItem _founditeminslot)))) (.Icon (Utilities|Struct|BreakS_Item (Variables|/Game/GatheringResourcesSystem/UI/Widgets/WBP_InventorySlot.WBP_InventorySlot_C|GetItem _founditeminslot)))) _founditeminslot))
    (:Is%20Not%20Valid
      (bind _potentialfreeslot (Private|FindFirstFreeSlotinInventory))
      (Utilities|IsValid _potentialfreeslot
        (:Is%20Valid
          (Private|ShowIteminInventorySlot (Variables|Default|GetItem%20to%20Add) _potentialfreeslot))
        (:Is%20Not%20Valid
          (Development|PrintString "No space in your inventory"))))))

(fn InitializeInventory
  (params (OverlayInventoryTarget :type Overlay%20Object%20Reference) (OwningPlayer :type Player%20Controller%20Object%20Reference))
  (bind _returnvalue (UserInterface|CreateWidget "/Game/GatheringResourcesSystem/UI/Widgets/WBP_Inventory.WBP_Inventory_C" OwningPlayer))
  (bind _output_get (Variables|Default|SetREF_Inventory _returnvalue))
  (Class|Overlay|AddChildtoOverlay OverlayInventoryTarget _output_get)
  (Variables|Default|SetInventory%20Slots (Variables|/Game/GatheringResourcesSystem/UI/Widgets/WBP_Inventory.WBP_Inventory_C|GetInventorySlots _output_get))
  (return))

(fn FindifThereIsSameItem
  (params (ItemToAdd :type S%20Item%20Structure))
  (bind (_name _tier) (Utilities|Struct|BreakS_Item ItemToAdd))
  (bind _array_element (Utilities|Array|ForEachLoopwithBreak (Variables|Default|GetInventory%20Slots) :!label _label)
    (:LoopBody
      (LocalVariables|SetLOCAL_FoundItemInSlot _array_element)
      (if (and (Utilities|Enum|Equal(Enum) (.Name (Utilities|Struct|BreakS_Item (Variables|/Game/GatheringResourcesSystem/UI/Widgets/WBP_InventorySlot.WBP_InventorySlot_C|GetItem _array_element))) _name) (== (.Tier (Utilities|Struct|BreakS_Item (Variables|/Game/GatheringResourcesSystem/UI/Widgets/WBP_InventorySlot.WBP_InventorySlot_C|GetItem _array_element))) _tier))
        (goto _label Break)
        (else
          (LocalVariables|SetLOCAL_FoundItemInSlot 0))))
    (:Completed
      (return (LocalVariables|GetLOCAL_FoundItemInSlot)))))

(fn ShowIteminInventorySlot
  (params (ItemToAdd :type S%20Item%20Structure) (InventorySlot :type WBP%20Inventory%20Slot%20Object%20Reference))
  (Variables|/Game/GatheringResourcesSystem/UI/Widgets/WBP_InventorySlot.WBP_InventorySlot_C|SetItem InventorySlot ItemToAdd)
  (Default|UpdateItem InventorySlot)
  (return))

(fn FindFirstFreeSlotinInventory
  (bind _array_element (Utilities|Array|ForEachLoopwithBreak (Variables|Default|GetInventory%20Slots) :!label _label)
    (:LoopBody
      (if (Utilities|Array|IsEmpty (.Name (Utilities|Struct|BreakS_Item (Variables|/Game/GatheringResourcesSystem/UI/Widgets/WBP_InventorySlot.WBP_InventorySlot_C|GetItem _array_element))))
        (LocalVariables|SetLOCAL_EmptyInventorySlot _array_element)
        (goto _label Break)
        (else
          (LocalVariables|SetLOCAL_EmptyInventorySlot 0))))
    (:Completed
      (return (LocalVariables|GetLOCAL_EmptyInventorySlot)))))