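; Actor component that manages a player's equipped gathering tool, its access tags and the montage matching its type.
; Equipping stores the tool, adds its gameplay tags for gatherability checks and attaches it to a mesh socket; detaching, optionally ground-checked, or durability loss clears it.
; RepNotifies update a local-only tool widget's icon and durability bar.
; BeginPlay resolves the pawn from a PlayerState or Pawn owner with retry macros.
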(event Custom|Server_DetatchToolFromPlayer
  (Utility|DetachToolfromPlayer true))

(event Custom|Owning_SetToolWidget
  (params (InVisibility :type ESlateVisibility%20Enum :default "Visible") (LocalPlayerController :type Player%20Controller%20Object%20Reference))
  (bind _toolwidget (Variables|Default|GetToolWidget))
  (Widget|SetVisibility _toolwidget InVisibility)
  (Class|UserWidget|SetOwningPlayer _toolwidget LocalPlayerController))

(event EventBeginPlay
  (bind _ownerpawn (Variables|Default|GetOwnerPawn))
  (if (.bSuccess (Utilities|Casting|CastToPlayerState (Components|GetOwner)))
    (Utilities|GetPawnfromState 10
      (:failed
        (Development|PrintString "GettingPawnFailed" :!label _label))
      (:succes
        (if (Pawn|IsLocallyControlled _ownerpawn) :!label _label_2
          (bind _returnvalue (UserInterface|CreateWidget "/Game/GatheringResourcesSystem/UI/Widgets/WBP_Tool.WBP_Tool_C" (Pawn|GetLocalViewingPlayerController _ownerpawn)))
          (Variables|Default|SetToolWidget _returnvalue)
          (UserInterface|Viewport|AddtoViewport (Variables|Default|GetToolWidget) 0)
          (Widget|SetVisibility (Variables|Default|GetToolWidget) "Collapsed"))))
    (else
      (Utilities|GetPawnfromCharacter 10
        (:failed
          (goto _label))
        (:succes
          (goto _label_2))))))

(fn TryEquipGatheringTool
  (params (TargetPlayer :type Actor%20Object%20Reference%20%28by%20ref%29) (TagsToAdd :type Gameplay%20Tag%20Container%20Structure%20%28by%20ref%29) (GatheringToolToEquipp :type BP%20Gathering%20Tool%20Object%20Reference))
  (if (Utility|IsToolEquipped)
    (return false)
    (else
      (Seters|SetGatheringTool GatheringToolToEquipp)
      (Manipulating|AddGatheringAccesTags TagsToAdd)
      (Utility|AttatchTooltoPlayer TargetPlayer GatheringToolToEquipp)
      (CallFunction|OwningSetToolWidget "Visible")
      (return true))))

(fn AddGatheringAccesTags
  (params (Tags :type Gameplay%20Tag%20Container%20Structure%20%28by%20ref%29))
  (GameplayTags|AppendGameplayTagContainers (Variables|Default|GetGatheringAccesTags) Tags)
  (Variables|Default|SetTierOfCurrentTool (GameplayTags|GetNumGameplayTagsinContainer Tags))
  (return))

(fn RemoveGatheringAccesTags
  (params (TagsToRemove :type Gameplay%20Tag%20Container%20Structure))
  (for _array_element (GameplayTags|BreakGameplayTagContainer TagsToRemove)
    (GameplayTags|RemoveGameplayTag (Variables|Default|GetGatheringAccesTags) _array_element :!class /Script/GameplayTags.BlueprintGameplayTagLibrary))
  (return))

(fn DEBUGPrintAllTags
  (for _array_element (GameplayTags|BreakGameplayTagContainer (Variables|Default|GetGatheringAccesTags))
    (Development|PrintString (Utilities|String|ToString(Name) (GameplayTags|GetTagName _array_element)) true true "(R=1.000000,G=0.000000,B=0.033201,A=1.000000)")))

(fn DetachToolfromPlayer
  (params (useGroundCheck? :type Boolean))
  (bind _currentlyusingtool (Variables|Default|GetCurrentlyUsingTool)
    (:then
      (if useGroundCheck?
        (bind (_locationfound _location) (Default|FindGround _currentlyusingtool))
        (if _locationfound
          (Transformation|SetActorLocation _currentlyusingtool _location false false)
          (Transformation|DetachFromActor _currentlyusingtool "KeepWorld" "KeepRelative" "KeepWorld")
          (Default|Drop/HideTool _currentlyusingtool)
          (Utility|ClearGatheringTool)
          (return))
        (else
          (Transformation|DetachFromActor _currentlyusingtool "KeepWorld" "KeepRelative" "KeepWorld")
          (Default|Drop/HideTool _currentlyusingtool)
          (Utility|ClearGatheringTool)
          (return))))
    (:else)))

(fn AttatchTooltoPlayer
  (params (Target :type Actor%20Object%20Reference%20%28by%20ref%29) (ToolToEquipp :type Actor%20Object%20Reference%20%28by%20ref%29))
  (bind _pawnmesh (Class|BPIGetMesh|GetPawnMesh(Message) Target))
  (Transformation|AttachComponentToComponent ToolToEquipp _pawnmesh (Variables|Animations|GetGatheringToolSocketName) "SnapToTarget" "SnapToTarget" "SnapToTarget" false)
  (return))

(fn CanbeGathered?
  (params (Tag :type Gameplay%20Tag%20Structure))
  (return (Utility|CheckforGatheringAccesTags Tag)))

(fn IsToolEquipped
  (return (Utilities|IsValid (Variables|Default|GetCurrentlyUsingTool))))

(fn ClearGatheringTool
  (Manipulating|RemoveGatheringAccesTags (Default|GetToolAccesTags (Variables|Default|GetCurrentlyUsingTool)))
  (EventDispatchers|UnbindallEventsfromOnDurabilityLoss (Variables|Default|GetCurrentlyUsingTool))
  (EventDispatchers|UnbindallEventsfromOnDurabilityChange (Variables|Default|GetCurrentlyUsingTool))
  (Variables|Default|SetCurrentlyUsingTool 0)
  (Variables|Default|SetGatheringType "NewEnumerator4")
  (CallFunction|OwningSetToolWidget "Collapsed")
  (return))

(fn CheckforGatheringAccesTags
  (params (Tag :type Gameplay%20Tag%20Structure))
  (return (GameplayTags|HasTag (Variables|Default|GetGatheringAccesTags) Tag true)))

(fn SetGatheringTool
  (params (GatheringTool :type BP%20Gathering%20Tool%20Object%20Reference%20%28by%20ref%29))
  (EventDispatchers|BindEventtoOnDurabilityLoss GatheringTool (EventDispatchers|CreateEvent :!event BINDonDurabilityToolLoss))
  (EventDispatchers|BindEventtoOnDurabilityChange GatheringTool (EventDispatchers|CreateEvent :!event BINDonDurabilityChange))
  (bind _output_get (Variables|Default|SetCurrentlyUsingTool GatheringTool))
  (Variables|Default|SetGatheringType (Default|GetType _output_get))
  (return))

(fn GetTool
  (return (Variables|Default|GetCurrentlyUsingTool)))

(fn GetGatheringAnimation
  (bind _gatheringtype (Variables|Default|GetGatheringType))
  (bind _gatheringstonemontage (Variables|Animations|GetGatheringStoneMontage))
  (bind _gatheringgoldmontage (Variables|Animations|GetGatheringGoldMontage))
  (bind _gatheringcrystalmontage (Variables|Animations|GetGatheringCrystalMontage))
  (bind _returnvalue (Utilities|Select :Index _gatheringtype :NewEnumerator4 0 :NewEnumerator0 _gatheringstonemontage :NewEnumerator1 _gatheringcrystalmontage :NewEnumerator3 _gatheringgoldmontage))
  (if (Utilities|IsValid (Variables|Default|GetCurrentlyUsingTool))
    (if (Utilities|IsValid _returnvalue)
      (return _returnvalue)
      (else
        (Development|PrintString (Utilities|String|Append (Utilities|String|EnumtoString (Variables|Default|GetGatheringType)) " : Animation " "is not valid. Please set animation for this action in BPC_GatheringComponent."))
        (return _returnvalue)))
    (else
      (return 0))))

(fn GetToolTier
  (return (Variables|Default|GetTierOfCurrentTool)))

(fn BINDonDurabilityToolLoss
  (Utility|ClearGatheringTool)
  (return))

(fn BINDonDurabilityChange
  (params (CurrentDurability :type Integer))
  (Variables|Default|SetCurrentToolDurability CurrentDurability))

(fn OnRepCurrentToolDurability
  (if (Pawn|IsLocallyControlled (Variables|Default|GetOwnerPawn))
    (Default|UpdatePB (Variables|Default|GetToolWidget) (Math|Conversions|ToFloat(Integer) (Variables|Default|GetCurrentToolDurability)))))

(fn OnRepCurrentlyUsingTool
  (bind _currentlyusingtool (Variables|Default|GetCurrentlyUsingTool))
  (bind _toolwidget (Variables|Default|GetToolWidget))
  (if (Pawn|IsLocallyControlled (Variables|Default|GetOwnerPawn))
    (Utilities|IsValid _currentlyusingtool
      (:Is%20Valid
        (Default|UpdatePB _toolwidget (Math|Conversions|ToFloat(Integer) (Default|GetDurabilityPercentage _currentlyusingtool)))
        (Default|UpdateIcon _toolwidget (Default|GetToolICon _currentlyusingtool))
        (return))
      (:Is%20Not%20Valid
        (return)))))