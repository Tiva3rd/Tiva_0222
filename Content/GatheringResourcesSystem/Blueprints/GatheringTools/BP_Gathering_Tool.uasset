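; Replicated gathering tool actor, configured by a data asset, that players pick up and use on interactable resources.
; On the server, overlapping its pickup sphere equips it through the player's gathering component with access tags, and dropping reverses this.
; Contact box overlaps trigger a box trace that sends an interaction message with hit details; animation start/end functions toggle that box.
; Durability changes are broadcast, and the tool is destroyed at zero.
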(event OnComponentBeginOverlap(OnContactBox)
  (params (OverlappedComponent :type Primitive%20Component%20Object%20Reference) (OtherActor :type Actor%20Object%20Reference) (OtherComp :type Primitive%20Component%20Object%20Reference) (OtherBodyIndex :type Integer) (bFromSweep :type Boolean) (SweepResult :type Hit%20Result%20Structure%20%28by%20ref%29))
  (if (> (Variables|Default|GetCurrentDurability) 0)
    (Utility|GatheringToolDetailedInteract OtherActor)
    (else
      (Development|PrintString "Your Tool require repair."))))

(event Custom|Owning_OnDurabilityChange
  (Default|CallOnDurabilityChange (Utility|GetDurabilityPercentage)))

(event Custom|Server_GatheringToolInteract
  (params (TestObject :type Object%20Object%20Reference))
  (CallFunction|OwningGatheringToolInteract TestObject))

(event Custom|Owning_GatheringToolInteract
  (params (TestObject :type Object%20Object%20Reference))
  (Utility|GatheringToolDetailedInteract TestObject))

(event EventBeginPlay
  (Networking|SwitchHasAuthority
    (:Authority
      (Collision|SetCollisionEnabled (Variables|Default|GetPickupSphere) "QueryOnly")
      (Collision|BindEventtoOnComponentBeginOverlap (Variables|Default|GetPickupSphere) (delegate Overlap_PickupSphere)))))

(event EventTick
  (params (DeltaSeconds :type Float%20%28single-precision%29)))

(fn ConstructionScript
  (Components|StaticMesh|SetStaticMesh (Variables|Default|GetSM_Gathering_Tool) (Variables|/Game/GatheringResourcesSystem/Blueprints/GatheringTools/DataAssets/PDA_Gathering_Tools.PDA_Gathering_Tools_C|GetStaticMesh (Variables|Default|GetDataAsset)))
  (Variables|Default|SetCurrentDurability (Variables|/Game/GatheringResourcesSystem/Blueprints/GatheringTools/DataAssets/PDA_Gathering_Tools.PDA_Gathering_Tools_C|GetDurability (Variables|Default|GetDataAsset))))

(fn OnRepVFXVisibility
  (if (Variables|Default|GetVFXVisibility)
    (Utility|ShowVFX)
    (else
      (Utility|HideVFX))))

(fn FindGround
  (bind _sm_indicatorcircle (Variables|Default|GetSM_IndicatorCircle))
  (bind _returnvalue (Transformation|GetWorldLocation _sm_indicatorcircle))
  (bind (_outhit _returnvalue_2) (Collision|LineTraceByChannel _returnvalue (+ _returnvalue (* (Math|Vector|VectorDown) 3e+02)) "TraceTypeQuery1" false (Utilities|Array|MakeArray (Components|GetOwner) 0) "None"))
  (if _returnvalue_2
    (return true (+ (.Location (Collision|BreakHitResult _outhit)) "0,0,10.000000"))
    (else
      (return false "0, 0, 0"))))

(fn GatheringToolDetailedInteract
  (params (TestObject :type Object%20Object%20Reference))
  (bind (_tracestart _traceend) (Utility|GetTraceLocations))
  (if (Utilities|DoesObjectImplementInterface TestObject "/Game/GatheringResourcesSystem/Blueprints/Interfaces/BPI_Interaction.BPI_Interaction_C")
    (bind (_outhit _returnvalue) (Collision|BoxTraceByChannel _tracestart _traceend "10.000000,10.000000,10.000000" "0, 0, 0" "TraceTypeQuery1" false (Utilities|Array|MakeArray (Components|GetOwner)) (Variables|Default|GetBoxTraceDebug)))
    (if _returnvalue
      (Class|BPIInteraction|DetailedInteract(Message) (.HitActor (Collision|BreakHitResult _outhit)) (.AsPawn (Utilities|Casting|CastToPawn (Components|GetOwner))) (.ImpactPoint (Collision|BreakHitResult _outhit)) (.ImpactNormal (Collision|BreakHitResult _outhit))))))

(fn Drop/HideTool
  (Networking|SwitchHasAuthority
    (:Authority
      (Variables|Default|SetVFXVisibility true)
      (Collision|SetCollisionEnabled (Variables|Default|GetPickupSphere) "QueryOnly")
      (bind _gatheringcomponent (Class|BPIGetComponents|GetGatheringComponent(Message) (Components|GetOwner)))
      (Default|RemoveGatheringAccesTags _gatheringcomponent (Variables|/Game/GatheringResourcesSystem/Blueprints/GatheringTools/DataAssets/PDA_Gathering_Tools.PDA_Gathering_Tools_C|GetGatheringTag (Variables|Default|GetDataAsset)))
      (Development|SetHiddeninGame (Variables|Default|GetSM_IndicatorCircle) false false)
      (Actor|SetOwner 0)
      (return))))

(fn GatheringAnimationStart
  (Networking|SwitchHasAuthority
    (:Authority
      (Collision|SetCollisionEnabled (Variables|Default|GetOnContactBox) "QueryOnly")
      (return))))

(fn GatheringAnimationEnd
  (Networking|SwitchHasAuthority
    (:Authority
      (Collision|SetCollisionEnabled (Variables|Default|GetOnContactBox) "NoCollision")
      (return))))

(fn OverrideAddtoInventory)

(fn ShowVFX
  (Rendering|SetVisibility (Variables|Default|GetVFX) true false)
  (Development|SetHiddeninGame (Variables|Default|GetSM_IndicatorCircle) false false)
  (return))

(fn HideVFX
  (Rendering|SetVisibility (Variables|Default|GetVFX) false false)
  (Development|SetHiddeninGame (Variables|Default|GetSM_IndicatorCircle) true false)
  (return))

(fn GetDurabilityPercentage
  (return (Math|Float|Round (* (/ (Variables|Default|GetCurrentDurability) (Variables|/Game/GatheringResourcesSystem/Blueprints/GatheringTools/DataAssets/PDA_Gathering_Tools.PDA_Gathering_Tools_C|GetDurability (Variables|Default|GetDataAsset))) 1e+02))))

(fn ChangeDurability
  (params (Delta :type Integer))
  (bind _output_get (Variables|Default|SetCurrentDurability (Math|Integer|Clamp(Integer) (+ (Variables|Default|GetCurrentDurability) Delta) 0 (Variables|/Game/GatheringResourcesSystem/Blueprints/GatheringTools/DataAssets/PDA_Gathering_Tools.PDA_Gathering_Tools_C|GetDurability (Variables|Default|GetDataAsset)))))
  (Default|CallOnDurabilityChange (Utility|GetDurabilityPercentage))
  (if (< (Utility|GetDurabilityPercentage) 30)
    (if (<= _output_get 0)
      (Default|CallOnDurabilityLoss)
      ;[0 0 0] What to do if durability hit 0
      (Utility|DurabilityLoss))))

(fn RepairTool(%)
  (params (NewDurability :type Integer))
  (Utility|ChangeDurability (* (/ NewDurability (Variables|/Game/GatheringResourcesSystem/Blueprints/GatheringTools/DataAssets/PDA_Gathering_Tools.PDA_Gathering_Tools_C|GetDurability (Variables|Default|GetDataAsset))) 100))
  (return))

(fn GetTraceLocations
  (return (Transformation|GetWorldLocation (Variables|Default|GetTrace_Start)) (Transformation|GetWorldLocation (Variables|Default|GetTrace_End))))

(fn GetType
  (return (Variables|/Game/GatheringResourcesSystem/Blueprints/GatheringTools/DataAssets/PDA_Gathering_Tools.PDA_Gathering_Tools_C|GetGatheringType (Variables|Default|GetDataAsset))))

(fn DurabilityLoss
  (Actor|DestroyActor)
  (return))

(fn GetToolAccesTags
  (return (Variables|/Game/GatheringResourcesSystem/Blueprints/GatheringTools/DataAssets/PDA_Gathering_Tools.PDA_Gathering_Tools_C|GetGatheringTag (Variables|Default|GetDataAsset))))

(fn GetToolICon
  (return (Variables|/Game/GatheringResourcesSystem/Blueprints/GatheringTools/DataAssets/PDA_Gathering_Tools.PDA_Gathering_Tools_C|GetIcon (Variables|Default|GetDataAsset))))

(event Custom|Bind_PickupSphereOverlap
  (params (OverlappedComponent :type Primitive%20Component%20Object%20Reference) (OtherActor :type Actor%20Object%20Reference) (OtherComp :type Primitive%20Component%20Object%20Reference) (OtherBodyIndex :type Integer) (bFromSweep :type Boolean) (SweepResult :type Hit%20Result%20Structure%20%28by%20ref%29))
  (if (Utilities|DoesObjectImplementInterface OtherActor "/Game/GatheringResourcesSystem/Blueprints/Interfaces/BPI_GetMesh.BPI_GetMesh_C")
    (bind (_gatheringcomponent _succed) (Class|BPIGetComponents|GetGatheringComponent(Message) OtherActor))
    (if _succed
      (bind _succed_2 (Default|TryEquipGatheringTool _gatheringcomponent OtherActor (Variables|/Game/GatheringResourcesSystem/Blueprints/GatheringTools/DataAssets/PDA_Gathering_Tools.PDA_Gathering_Tools_C|GetGatheringTag (Variables|Default|GetDataAsset)) self))
      (if _succed_2
        (Variables|Default|SetVFXVisibility false)
        (Collision|SetCollisionEnabled (Variables|Default|GetPickupSphere) "NoCollision")
        (Actor|SetOwner OtherActor)
        (else
          ;[0 0 0] Equiping failed only if player already have equipped the tool, override this function with your desired behaviour. Ideally it should check additionaly if player have equipped any type of accesable stuff. You can also remove Attaching part from "Try Equip Gathering Tool" and connect it with inventory so player will have acces to gather even if tool is just in inventory.
          (Utility|OverrideAddtoInventory))))))