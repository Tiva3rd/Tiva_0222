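; BP_Destroyed_Resource is the physics debris of a destroyed resource in the gathering system, shrinking its pieces from BeginPlay.
; The construction script spawns a static mesh component for each mesh in a data table row, simulating physics with configurable damping and ignoring Pawn, Visibility and Camera channels.
; A timeline scales the stored components by lerping between zero and their current scale, so the scaling compounds each update.
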(event EventBeginPlay
  ;[1 1 1] Shrinking animation while destroy
  (bind _newtrack_0 (Timeline|Timeline_0 Play)
    (:Update
      (for _array_element (Variables|Default|GetStaticMeshesReference)
        (Transformation|SetWorldScale3D _array_element (Math|Vector|Lerp(Vector) "0, 0, 0" (Transformation|GetWorldScale _array_element) _newtrack_0))))))

(fn ConstructionScript
  (bind _dt_destroyedmesh (Variables|Default|GetDT_DestroyedMesh))
  (bind (_datatable _rowname) (Utilities|Struct|BreakDataTableRowHandle _dt_destroyedmesh))
  ;[1 1 1] Loop through DataTable create all meshes assign and set physics and damping
  (bind _returnvalue (Utilities|GetDataTableRow _datatable _rowname)
    (:then
      (bind _array_element (Utilities|Array|ForEachLoopwithBreak (Utilities|Struct|BreakS_DestroyedResource _returnvalue))
        (:LoopBody
          (bind _returnvalue_2 (AddComponent|AddStaticMeshComponent false))
          (Components|StaticMesh|SetStaticMesh _returnvalue_2 _array_element)
          (Physics|SetSimulatePhysics _returnvalue_2 true)
          (Collision|SetCollisionResponsetoChannel _returnvalue_2 "ECC_Pawn" "ECR_Ignore")
          (Collision|SetCollisionResponsetoChannel _returnvalue_2 "ECC_Visibility" "ECR_Ignore")
          (Collision|SetCollisionResponsetoChannel _returnvalue_2 "ECC_Camera" "ECR_Ignore")
          (Class|PrimitiveComponent|SetLinearDamping _returnvalue_2 (Variables|Default|GetLinear%20Damping))
          (Class|PrimitiveComponent|SetAngularDamping _returnvalue_2 (Variables|Default|GetAngular%20Damping))
          (Utilities|Array|Add (Variables|Default|GetStaticMeshesReference) _returnvalue_2)
          (Variables|Default|SetStaticMeshesReference (Variables|Default|GetStaticMeshesReference)))))))