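; Base gatherable resource node for multiplayer, configured from a data table row chosen by resource name.
; On authority, BeginPlay sets HP, randomized yield and an enchantment tier (override or probability-based roll), whose OnRep drives tier VFX.
; Interaction checks the tool tag, costs durability and deals tool-tier damage, starting a bonus game while HP remains.
; Depletion or the bonus game callback adds the item to inventory and multicasts the destructible mesh swap.
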(event BonusGameRes(BPC_BonusGame)
  (params (MultiplicationValue :type Float%20%28double-precision%29) (GameResult :type E_GameResult%20Enum :default "NewEnumerator0"))
  ;[0 0 0] BonusGameCallback
  (CallFunction|DestroyResource MultiplicationValue))

(event EventTick
  (params (DeltaSeconds :type Float%20%28single-precision%29)))

(fn ConstructionScript
  (bind _resourcemesh (Variables|Default|GetResourceMesh))
  (bind _vfx_tier (Variables|Default|GetVFX_Tier))
  (bind (_origin _boxextent _sphereradius) (Collision|GetComponentBounds _resourcemesh))
  ;[0 0 0] get data from data table and assign mesh
  (bind _returnvalue (Utilities|GetDataTableRow (Variables|GatheringData|GetGatheringSystemData) (Utilities|String|StringToName (Utilities|String|EnumtoString (Variables|Gathering|GetResourceNames))))
    (:then
      (bind _output_get (Variables|GatheringData|SetGatheringDataRefernce _returnvalue))
      (Variables|GatheringData|SetTag%20to%20Gather (.TagToGather (Utilities|Struct|BreakS_Gathering_System _output_get)))
      (Components|StaticMesh|SetStaticMesh (Variables|Default|GetResourceMesh) (.StaticMesh (Utilities|Struct|BreakS_Gathering_System _output_get)))
      (Class|NiagaraComponent|SetVariablePosition _vfx_tier "MeshPosition" _origin)
      (Effects|Components|ParticleSystem|SetFloatParameter _vfx_tier "SphereRadius" (+ _sphereradius (Variables|Gathering|GetVFXBoundSize))))))

(fn SumProbability
  (bind _values (Utilities|Map|Values (.EnchantmentProbability (Utilities|Struct|BreakS_Gathering_System (Variables|GatheringData|GetGatheringDataRefernce)))))
  (for _array_element _values
    (LocalVariables|SetLOCAL_Sum (+ (LocalVariables|GetLOCAL_Sum) _array_element)))
  (return (LocalVariables|GetLOCAL_Sum)))

(fn TierChoose
  (params (Weighted%20Sum :type Float%20%28double-precision%29))
  (bind _values (Utilities|Map|Values (.EnchantmentProbability (Utilities|Struct|BreakS_Gathering_System (Variables|GatheringData|GetGatheringDataRefernce)))))
  (bind (_array_element _array_index) (Utilities|Array|ForEachLoopwithBreak _values :!label _label)
    (:LoopBody
      (bind _output_get (LocalVariables|SetLOCAL_WeightedSum (+ _array_element (LocalVariables|GetLOCAL_WeightedSum))))
      (if (>= _output_get (Math|Random|RandomFloatinRange 0.0 Weighted%20Sum))
        (goto _label Break)))
    (:Completed
      (return _array_index))))

(fn InitializeHP
  (bind _output_get (Variables|Utility|SetMaxHealth (.MaxHealth (Utilities|Struct|BreakS_Gathering_System (Variables|GatheringData|GetGatheringDataRefernce)))))
  (Variables|Utility|SetCurrentResourceHP _output_get)
  (return))

(fn InitializeResourceAmount
  (bind _multiplicationgatheredbonus (Variables|Gathering|GetMultiplicationGatheredBonus))
  (bind _gatheringdatarefernce (Variables|GatheringData|GetGatheringDataRefernce))
  (bind (_basegatheredamount _deltavarriationamount) (Utilities|Struct|BreakS_Gathering_System _gatheringdatarefernce))
  (Variables|Utility|SetResourceAmount (Math|Float|Round (* (+ (+ _basegatheredamount (* (Math|Random|RandomIntegerinRange 0 _deltavarriationamount) (Math|Integer|SelectInt 1 -1 (Math|Random|RandomBool)))) (Variables|Gathering|GetFlatGatheredBonus)) (Math|Float|SelectFloat 1.0 _multiplicationgatheredbonus (< _multiplicationgatheredbonus 1.0)))))
  (return))

(fn SpawnVFXonHit
  (params (Location :type Vector) (Normal :type Vector))
  (bind _returnvalue (Niagara|SpawnSystematLocation "/Game/GatheringResourcesSystem/VFX/N_OnHit.N_OnHit" Location))
  (Niagara|SetNiagaraVariable(Vector3) _returnvalue "MeshOrientation" Normal)
  (return))

(fn HideVFXifTier0
  (if (<= (Variables|GatheringData|GetEnchantmentThatWon) 0)
    (Rendering|SetVisibility (Variables|Default|GetVFX_Tier) false false)
    (return)
    (else
      (return))))

(fn CheckMatchingGameplayTag
  (params (TagToCheck :type Gameplay%20Tag%20Structure))
  (return false))

(fn ObtainHit
  (params (DamageDealt :type Integer))
  (bind _output_get (Variables|Utility|SetCurrentResourceHP (Math|Integer|Clamp(Integer) (- (Variables|Utility|GetCurrentResourceHP) DamageDealt) 0 (Variables|Utility|GetMaxHealth))))
  (return (<= _output_get 0)))

(fn OverrideEnchantment?
  (if (not (== (Variables|Gathering|GetOverrideEnchantment) -1))
    (return true)
    (else
      (return false))))

(fn SetRelatedDatatoVFX
  (bind _vfx_tier (Variables|Default|GetVFX_Tier))
  (Variables|Default|GetVFX_Tier
    (:then
      (Niagara|SetNiagaraVariable(LinearColor) _vfx_tier "Color" (CallFunction|BFLInterpEnchantment (Variables|GatheringData|GetEnchantmentThatWon)))
      (Class|NiagaraComponent|SetVariablePosition _vfx_tier "MeshPosition" (.Origin (Collision|GetComponentBounds (Variables|Default|GetResourceMesh))))
      (Rendering|SetVisibility _vfx_tier true false)
      (return))
    (:else)))

(fn GatheringDatatoItem
  (params (QuantityMultiplier :type Float%20%28double-precision%29))
  (bind _gatheringdatarefernce (Variables|GatheringData|GetGatheringDataRefernce))
  (bind (_name _icon) (Utilities|Struct|BreakS_Gathering_System _gatheringdatarefernce))
  (return (Utilities|Struct|MakeS_Item (Utilities|String|EnumtoString _name) (Variables|GatheringData|GetEnchantmentThatWon) (Math|Float|Round (* (Variables|Utility|GetResourceAmount) QuantityMultiplier)) _icon)))

(fn SpawnDestructableMeshandDestroyThis
  (bind _resourcemesh (Variables|Default|GetResourceMesh))
  (bind _resourcemesh_2 (Variables|Default|GetResourceMesh))
  (bind _returnvalue (Transformation|GetWorldTransform _resourcemesh))
  (Game|SpawnActorfromClass (.DestroyableMesh (Utilities|Struct|BreakS_Gathering_System (Variables|GatheringData|GetGatheringDataRefernce))) (Math|Transform|MakeTransform (.location _returnvalue) (.rotation _returnvalue) (.scale _returnvalue)) "AlwaysSpawn" self 3.0 0)
  (Development|SetHiddeninGame _resourcemesh_2 true false)
  (Collision|SetCollisionEnabled _resourcemesh_2 "NoCollision")
  (Actor|SetLifeSpan 5.0)
  (return))

(fn OnRepIsDestroyed
  (Private|SpawnDestructableMeshandDestroyThis)
  (return))

(fn DestroyResource
  (params (QuantityMultiplier :type Float%20%28double-precision%29))
  ;[0 0 0] For presentation purpose i decide once resource is destroyed, item should be added to inventory, if you want other behaviour like spawn object so anyone can pick it up do it here or simply swap with your own inventory.
  (bind _inventorycomponent (Class|BPIGetComponents|GetInventoryComponent(Message) (Variables|Utility|GetInstigatorPawn)))
  (Default|OwningTryAddItem _inventorycomponent (Private|GatheringDatatoItem QuantityMultiplier))
  (CallFunction|OwningShowGatheredAmountText QuantityMultiplier)
  (CallFunction|MultiPlayonDestroySound (Variables|Utility|GetHitLocation))
  (CallFunction|ServerSpawnDestructedandDestroy)
  (return))

(fn CreateCantbeGatheredNotify
  (if (not (Variables|Utility|GetNotificationWidgetCreated))
    (Variables|Utility|SetNotificationWidgetCreated true)
    (bind _returnvalue (Utilities|Time|SetTimerbyFunctionName 0 "StartNotificationWidgetTimer" (Variables|Utility|GetNotificationWidgetCooldownTimer)))
    (Variables|Utility|SetStartNotificationWidgetTimer_Handler _returnvalue)
    (bind _returnvalue_2 (UserInterface|CreateWidget "/Game/GatheringResourcesSystem/UI/Widgets/WBP_Notification.WBP_Notification_C" 0 "You don't have tool to gather it."))
    (UserInterface|Viewport|AddtoViewport _returnvalue_2 0)
    (return)))

(fn StartNotificationWidgetTimer
  (Variables|Utility|SetNotificationWidgetCreated false)
  (Utilities|Time|ClearandInvalidateTimerbyHandle (Variables|Utility|GetStartNotificationWidgetTimer_Handler))
  (return))

(fn OnRepEnchantmentThatWon
  (Private|SetRelatedDatatoVFX)
  (Private|HideVFXifTier0)
  (return))

(fn CreateGatheredAmountWidget
  (bind _returnvalue (UserInterface|CreateWidget "/Game/GatheringResourcesSystem/UI/Widgets/WBP_GatheredAmountNotification.WBP_GatheredAmountNotification_C" 0 (Utilities|Text|ToText(Integer) (Variables|Utility|GetResourceAmount)) (Utilities|Text|ToText(String) (Utilities|String|EnumtoString (Variables|Gathering|GetResourceNames)))))
  (bind _output_get (Variables|Utility|SetGatheredNotificationWidget _returnvalue))
  (UserInterface|SetWidget (Variables|Default|GetGatheredAmountWidget) _output_get)
  (return))

(fn CalculatedDurabilityLoss
  (params (ToolTier :type Integer))
  (return (* (Math|Integer|Clamp(Integer) (- (* (.ResourceTier (Utilities|Struct|BreakS_Gathering_System (Variables|GatheringData|GetGatheringDataRefernce))) 2) ToolTier) 1 99) -1)))

(fn UpdateDebugWidget
  (params (ShowDebug? :type Boolean))
  (bind _debugwidget (Variables|Default|GetDebugWidget))
  (Development|SetHiddeninGame _debugwidget (not ShowDebug?) false)
  (bind _aswbp_debug_resource (Utilities|Casting|CastToWBP_DebugResource (UserInterface|GetWidget _debugwidget)))
  (Default|InitDebugResource _aswbp_debug_resource (Utilities|Text|ToText(Integer) (Variables|Utility|GetCurrentResourceHP)) (Utilities|Text|ToText(String) (Utilities|String|EnumtoString (.Name (Utilities|Struct|BreakS_Gathering_System (Variables|GatheringData|GetGatheringDataRefernce))))) (Variables|GatheringData|GetEnchantmentThatWon) (Components|GetOwner)))

(event EventDetailedInteract
  (params (InstigatorPawn :type Pawn%20Object%20Reference%20%28by%20ref%29) (HitLocation :type Vector%20%28by%20ref%29 :default "0, 0, 0") (HitNormal :type Vector%20%28by%20ref%29 :default "0, 0, 0"))
  (if (not (Default|GetIsBonusGameRunning? (Variables|Default|GetBPC_BonusGame)))
    (Variables|Utility|SetInstigatorPawn InstigatorPawn)
    (bind (_gatheringcomponent _succed) (Class|BPIGetComponents|GetGatheringComponent(Message) InstigatorPawn))
    (if _succed
      (bind _succed_2 (Default|CanbeGathered? _gatheringcomponent (Variables|GatheringData|GetTag%20to%20Gather)))
      (if _succed_2
        (Variables|Utility|SetHitLocation HitLocation)
        (Default|ChangeDurability (Default|GetTool _gatheringcomponent) -10)
        (CallFunction|MultiPlayonHitSound HitLocation)
        (CallFunction|MultiSpawnVFXonHit HitLocation HitNormal)
        (bind _isdestroyed_ (Private|ObtainHit (Default|GetToolTier _gatheringcomponent)))
        (if _isdestroyed_
          (Actor|SetOwner (Variables|Utility|GetInstigatorPawn))
          (CallFunction|DestroyResource 1.0)
          (else
            (Default|TryStartBonusGame (Variables|Default|GetBPC_BonusGame) InstigatorPawn (Pawn|GetController InstigatorPawn))))
        (else
          (CallFunction|MultiCreateCantbeGatheredNotify)))
      (else
        (Development|PrintString "Invalid  
Gathering 
 Component")))))

(event Custom|Multi_CreateCantBeGatheredNotify
  ;[0 0 0] Cosmetics
  (if (Pawn|IsLocallyControlled (Variables|Utility|GetInstigatorPawn))
    (CallFunction|CreateCantbeGatheredNotify)))

(event Custom|Multi_SpawnVFXOnHit
  (params (Location :type Vector) (Normal :type Vector))
  ;[0 0 0] Cosmetics
  (Private|SpawnVFXonHit Location Normal))

(event Custom|Server_SpawnDestructedAndDestroy
  ;[0 0 0] Cosmetics
  (CallFunction|MultiSpawnDestructedandDestroy))

(event Custom|Multi_PlayOnDestroySound
  (params (Location :type Vector))
  ;[0 0 0] Cosmetics
  (Audio|PlaySoundatLocation (.OnDestroySound (Utilities|Struct|BreakS_Gathering_System (Variables|GatheringData|GetGatheringDataRefernce))) Location "0, 0, 0" 1.0 1.0 0.0 0 0 0 0))

(event Custom|Owning_ShowGatheredAmountText
  (params (Multiplier :type Float%20%28double-precision%29))
  ;[0 0 0] Cosmetics
  (Default|PlayinAnimation (Variables|Utility|GetGatheredNotificationWidget) (Utilities|Text|ToText(Integer) (Math|Float|Round (* Multiplier (Variables|Utility|GetResourceAmount))))))

(event Custom|Multi_PlayOnHitSound
  (params (Location :type Vector))
  ;[0 0 0] Cosmetics
  (Audio|PlaySoundatLocation (.OnHitSound (Utilities|Struct|BreakS_Gathering_System (Variables|GatheringData|GetGatheringDataRefernce))) Location "0, 0, 0" 1.0 1.0 0.0 0 0 0 0))

(event Custom|Multi_SpawnDestructedAndDestroy
  ;[0 0 0] Cosmetics
  (Private|SpawnDestructableMeshandDestroyThis))

(event EventBeginPlay
  (CallFunction|CreateGatheredAmountWidget)
  (Networking|SwitchHasAuthority
    (:Authority
      (Private|InitializeHP)
      (Private|InitializeResourceAmount)
      (if (Private|OverrideEnchantment?)
        (Variables|GatheringData|SetEnchantmentThatWon (Variables|Gathering|GetOverrideEnchantment))
        (else
          (bind _weightedsum (Private|SumProbability))
          (bind _indexthatwon (Private|TierChoose _weightedsum))
          (Variables|GatheringData|SetEnchantmentThatWon _indexthatwon))))))