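; BP_BonusGameIndicator is an actor in the gathering resources system that hosts the bonus game appearance indicator.
; On BeginPlay it creates the indicator widget from a class variable, sets it on its widget component and caches it as WBP_BonusGameAppear.
; It binds to the widget's animation-end event to destroy itself.
; A separate onDestroy event tells the widget to destroy its indicator.
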(event Custom|Bind_BonusGameAnimationEnd
  (Actor|DestroyActor))

(event Custom|onDestroy
  (Default|DestroyWidgetIndicator (Variables|Default|GetWBP_BonusGameIndicator)))

(event EventBeginPlay
  (bind _bonusgameindicator (Variables|Default|GetBonusGameIndicator))
  (bind _returnvalue (UserInterface|CreateWidget (Variables|Default|GetWidgetIndicatorClass)))
  (UserInterface|SetWidget _bonusgameindicator _returnvalue)
  (bind _aswbp_bonus_game_appear (Utilities|Casting|CastToWBP_BonusGameAppear (UserInterface|GetUserWidgetObject _bonusgameindicator)))
  (bind _output_get (Variables|Default|SetWBP_BonusGameIndicator _aswbp_bonus_game_appear))
  (EventDispatchers|BindEventtoBonusGameAnimationEnd _output_get (delegate Custom|Bind_BonusGameAnimationEnd)))

(fn ConstructionScript)