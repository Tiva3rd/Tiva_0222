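; Player controller for the gathering resources system that sets up the inventory UI and input modes.
; On BeginPlay it forces fullscreen, then polls for the HUD and player UI through delayed DoN retry loops before initializing the showcase inventory component.
; The I key toggles the inventory overlay on the local player.
; Helpers switch cursor and input mode and fetch the gathering component from PlayerState, while GetInventoryComponent is a stub returning failure.
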(event EventBeginPlay
  (bind _returnvalue (Settings|GetGameUserSettings))
  (Class|GameUserSettings|SetFullscreenMode _returnvalue "Fullscreen")
  (Utilities|TrytoGetHUDnTimes 10
    (:Success
      (bind _ref_playerui (Utilities|TrytoGetPlayerInventory)
        (:Success
          (Default|InitializeInventory (Variables|Default|GetBPC_ShowcaseInventory) (Variables|/Game/GatheringResourcesSystem/UI/Widgets/WBP_PlayerUI.WBP_PlayerUI_C|GetOV_Inventory _ref_playerui) self))))))

(event Input|KeyboardEvents|I
  (params (Key :type Key%20Structure :default "None"))
  (bind _as_bp_my_hud (Variables|Default|GetAs%20BP%20My%20HUD))
  (bind _ref_playerui (Variables|/Game/GatheringResourcesSystem/Framework/BP_MyHUD.BP_MyHUD_C|GetREF_PlayerUI _as_bp_my_hud))
  (bind _ov_inventory (Variables|/Game/GatheringResourcesSystem/UI/Widgets/WBP_PlayerUI.WBP_PlayerUI_C|GetOV_Inventory _ref_playerui))
  ;[0 0 0] Flip inventory visibility
  (:Pressed
    (if (Pawn|IsLocalPlayerController)
      (Widget|SetVisibility _ov_inventory (select (Widget|IsVisible _ov_inventory) "Collapsed" "SelfHitTestInvisible")))))

(fn ConstructionScript)

(fn GetPlayerUI
  (bind _ref_playerui (Variables|/Game/GatheringResourcesSystem/Framework/BP_MyHUD.BP_MyHUD_C|GetREF_PlayerUI (Variables|Default|GetAs%20BP%20My%20HUD))
    (:then
      (return _ref_playerui))
    (:else)))

(fn SetMode
  (params (Show%20Mouse%20Cursor :type Boolean) (InWidgetToFocus :type Widget%20Object%20Reference))
  (bind _output_get (Variables|Default|SetbShowMouseCursor Show%20Mouse%20Cursor))
  (if _output_get
    (Input|SetInputModeGameandUI self InWidgetToFocus "DoNotLock" true false)
    (return)
    (else
      (Input|SetInputModeGameOnly self false)
      (return))))

(fn GetGatheringComponent
  (bind _playerstate (Variables|GetPlayerState))
  (bind _returnvalue (Actor|GetComponentbyClass _playerstate "/Game/GatheringResourcesSystem/Blueprints/BlueprintComponents/BPAC_GatheringComponent.BPAC_GatheringComponent_C"))
  (return _returnvalue (Utilities|IsValid _returnvalue)))

(fn GetInventoryComponent
  (return false 0))