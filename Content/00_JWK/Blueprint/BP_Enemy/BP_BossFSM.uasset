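; Boss enemy state machine component that drives its BP_Enemy_Boss owner against the player character.
; Tick switches on State: Idle caches the player and owner, then Move steers straight toward the target with movement input until within AttackDis.
; Attack only waits briefly and returns to Move when the 2D distance reaches AttackDis; it performs no attack action.
; The current state prints every tick.
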(event EventBeginPlay)

(event EventTick
  (params (DeltaSeconds :type Float%20%28single-precision%29))
  (bind _returnvalue (Game|GetPlayerCharacter 0))
  (Development|PrintString (Utilities|String|EnumtoString (Variables|Default|GetState)))
  (switch Utilities|FlowControl|Switch|SwitchonBP_Boss_Enemy (Variables|Default|GetState)
    (:NewEnumerator0
      ;[1 0 0] Idle
      (Utilities|IsValid _returnvalue
        (:Is%20Valid
          (Variables|Default|Settarget _returnvalue)
          (bind _asbp_enemy_boss (Utilities|Casting|CastToBP_Enemy_Boss (Components|GetOwner)))
          (Variables|Default|Setme _asbp_enemy_boss)
          (Variables|Default|SetState "NewEnumerator1"))))
    (:NewEnumerator1
      ;[0 1 0] Move
      (Pawn|Input|AddMovementInput (Variables|Default|Getme) (- (Transformation|GetActorLocation (Variables|Default|Gettarget)) (Transformation|GetActorLocation (Variables|Default|Getme))) 1.0 false)
      (if (< (Math|Vector|VectorLength (- (Transformation|GetActorLocation (Variables|Default|Gettarget)) (Transformation|GetActorLocation (Variables|Default|Getme)))) (Variables|Default|GetAttackDis))
        (Variables|Default|SetState "NewEnumerator2")))
    (:NewEnumerator2
      ;[0 0 1] Attack
      (Utilities|FlowControl|Delay 0.2)
      (if (>= (Math|Vector|Distance2D(Vector) (Transformation|GetActorLocation (Variables|Default|Gettarget)) (Transformation|GetActorLocation (Variables|Default|Getme))) (Variables|Default|GetAttackDis))
        (Variables|Default|SetState "NewEnumerator1")))))