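; Boss enemy Blueprint that deals damage to the archer player and registers sword hits on the house's target columns.
; Sword overlaps with a column increment a hit counter, which sets a house-hit flag once it passes a threshold.
; The attack sphere damages BP_Archer on end overlap rather than begin overlap.
; DealAttack is an empty event, and the sphere-overlap area-damage logic with debug drawing is disconnected and never runs.
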(event OnComponentEndOverlap(attackSphereComp)
  (params (OverlappedComponent :type Primitive%20Component%20Object%20Reference) (OtherActor :type Actor%20Object%20Reference) (OtherComp :type Primitive%20Component%20Object%20Reference) (OtherBodyIndex :type Integer))
  (bind _asbp_archer (Utilities|Casting|CastToBP_Archer OtherActor))
  (Class|TivaCharacter|PlayerTakeDamaged _asbp_archer 10))

(event OnComponentBeginOverlap(swordComp)
  (params (OverlappedComponent :type Primitive%20Component%20Object%20Reference) (OtherActor :type Actor%20Object%20Reference) (OtherComp :type Primitive%20Component%20Object%20Reference) (OtherBodyIndex :type Integer) (bFromSweep :type Boolean) (SweepResult :type Hit%20Result%20Structure%20%28by%20ref%29))
  (Utilities|Casting|CastToBP_houseTargetColumn OtherActor)
  (bind _output_get (Variables|Default|SetHItCount (+ (Variables|Default|GetHItCount) 1.0)))
  (if (> _output_get 15.0)
    (Variables|Default|SetHitHouseBoos true)))

(event Custom|DealAttack)

(event EventBeginPlay)

(event Collision|EventActorBeginOverlap
  (params (OtherActor :type Actor%20Object%20Reference)))

(event EventTick
  (params (DeltaSeconds :type Float%20%28single-precision%29)))

(fn ConstructionScript)