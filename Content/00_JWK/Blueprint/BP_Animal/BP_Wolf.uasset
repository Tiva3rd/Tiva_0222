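; BP_Wolf is a wolf animal that damages BP_Archer players through its AttackComp overlap volume.
; Damage fires when an archer's overlap with AttackComp ends, not when it begins, alongside a debug print.
; A C2S event skips dead players and forwards to an S2M event, named as a client-to-server-to-multicast relay.
; The S2M event applies fixed damage and triggers the player's death once HP runs out.
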(event OnComponentEndOverlap(attackComp)
  (params (OverlappedComponent :type Primitive%20Component%20Object%20Reference) (OtherActor :type Actor%20Object%20Reference) (OtherComp :type Primitive%20Component%20Object%20Reference) (OtherBodyIndex :type Integer))
  (Development|PrintString "Wolf Attacking!!!")
  (bind _asbp_archer (Utilities|Casting|CastToBP_Archer OtherActor))
  (CallFunction|PlayerDamageC2S _asbp_archer))

(event Custom|PlayerDamage_S2M
  (params (NewParam :type BP%20Archer%20Object%20Reference))
  (bind _playerhp (Variables|/Script/Tiva.TivaCharacter|GetplayerHP NewParam))
  (bind _returnvalue (<= _playerhp 0.0))
  (Class|TivaCharacter|PlayerTakeDamaged NewParam 2)
  (if _returnvalue
    (Default|PlayerDead NewParam _returnvalue)))

(event Custom|PlayerDamage_C2S
  (params (NewParam :type BP%20Archer%20Object%20Reference))
  (if (not (Variables|/Game/00_NYJ/Character/BP_Archer.BP_Archer_C|GetisDead? NewParam))
    (CallFunction|PlayerDamageS2M NewParam)))

(event EventBeginPlay)

(event Collision|EventActorBeginOverlap
  (params (OtherActor :type Actor%20Object%20Reference)))

(event EventTick
  (params (DeltaSeconds :type Float%20%28single-precision%29)))

(fn ConstructionScript)