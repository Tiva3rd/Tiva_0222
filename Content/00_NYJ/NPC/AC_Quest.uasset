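; Quest component that drives NPC dialogue UI and tracks the player's quest state.
; The archer-to-NPC interaction casts the NPC to Bp_enemySolder and picks its UI by quest state, with a one-shot IsDone flag selecting the meet message.
; Setting the state also copies it to the BP_Archer pawn cached at BeginPlay.
; NPC-to-archer interaction and item confirmation are empty stubs.
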(event EventBeginPlay
  (bind _asbp_archer (Utilities|Casting|CastToBP_Archer (Game|Player|GetPlayerPawn 0)))
  (Variables|Default|SetAs%20BP%20Archer _asbp_archer))

(event EventTick
  (params (DeltaSeconds :type Float%20%28single-precision%29)))

(fn FInteractionAtoN
  (params (CurrentState :type E_QuestState%20Enum :default "NewEnumerator0") (NPC :type Actor%20Object%20Reference))
  (bind _output_get (Variables|Default|SetCurrent%20State CurrentState))
  (bind _asbp_enemy_solder (Utilities|Casting|CastToBp_enemySolder NPC))
  (Variables|Default|SetAs%20Bp%20Enemy%20Solder _asbp_enemy_solder)
  (switch Utilities|FlowControl|Switch|SwitchonE_QuestState _output_get
    (:NewEnumerator0
      (if (Variables|Default|GetIsDone?)
        (Variables|Default|SetIsDone? false)
        (Default|ShowMessageUINpcMeet (Variables|Default|GetAs%20Bp%20Enemy%20Solder))
        (else
          (Default|ShowUI1st (Variables|Default|GetAs%20Bp%20Enemy%20Solder)))))
    (:NewEnumerator1
      (Default|ShowUI2nd (Variables|Default|GetAs%20Bp%20Enemy%20Solder)))))

(fn FInteractionNtoA)

(fn FConfirmItem
  (params (OverlapItem :type Actor%20Object%20Reference)))

(fn FSetStateQuest
  (params (NewQuestState :type E_QuestState%20Enum :default "NewEnumerator0"))
  (bind _output_get (Variables|Default|SetCurrent%20State NewQuestState))
  (Variables|/Game/00_NYJ/Character/BP_Archer.BP_Archer_C|SetState_Quest (Variables|Default|GetAs%20BP%20Archer) _output_get))