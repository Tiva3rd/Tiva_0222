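; BP_MyCharacter_Tiva is a player character Blueprint that adds the WBP_Aim widget to the viewport on BeginPlay.
; It holds an unconnected bow-fire chain, gated by CanFire, that traces from the camera to find an aim point.
; That chain spawns BP_Arrow at the mesh's arrow socket, rotated toward that point so shots converge on the camera's aim, then plays a fire montage.
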(event EventBeginPlay
  (bind _returnvalue (UserInterface|CreateWidget "/Game/00_NYJ/Blueprint/WBP_Aim.WBP_Aim_C"))
  (UserInterface|Viewport|AddtoViewport _returnvalue 0))

(event Collision|EventActorBeginOverlap
  (params (OtherActor :type Actor%20Object%20Reference)))

(event EventTick
  (params (DeltaSeconds :type Float%20%28single-precision%29)))

(event Input|ActionEvents|InputActionFire
  (params (Key :type Key%20Structure :default "None")))

(fn ConstructionScript)