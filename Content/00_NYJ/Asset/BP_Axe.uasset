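; BP_Axe is an axe actor that applies hits to whatever its Collision component begins overlapping.
; Trees receive a chop message and spawn a chopping sphere above them; mines get an interface damage message and impact emitter.
; The mine branch tests the overlapped component's class rather than the other actor's.
; Boss and goblin hits damage the instance returned by GetActorOfClass, not necessarily the one struck.
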(event OnComponentBeginOverlap(Collision)
  (params (OverlappedComponent :type Primitive%20Component%20Object%20Reference) (OtherActor :type Actor%20Object%20Reference) (OtherComp :type Primitive%20Component%20Object%20Reference) (OtherBodyIndex :type Integer) (bFromSweep :type Boolean) (SweepResult :type Hit%20Result%20Structure%20%28by%20ref%29))
  (Utilities|FlowControl|Sequence
    (:then_0
      (if (== (Utilities|GetClass OverlappedComponent) "/Game/00_OJS/mining/MineActor.MineActor_C")
        (Utilities|Casting|CastToMineActor OtherActor)
        (Utilities|FlowControl|Sequence
          (:then_0
            (if (Utilities|DoesObjectImplementInterface OtherActor "/Game/00_OJS/ResourceGathering/Resource_BPI.Resource_BPI_C")
              (Class|ResourceBPI|DealDamage(Message) OtherActor)))
          (:then_1
            (Effects|SpawnEmitteratLocation 0 (Transformation|GetWorldLocation (Variables|Default|GetCollision)))))))
    (:then_1
      (if (== (Utilities|GetClass OtherActor) "/Game/00_OJS/tree/BP_ChoppalbeTree_OJS.BP_ChoppalbeTree_OJS_C")
        (bind _asbp_choppalbe_tree_ojs (Utilities|Casting|CastToBP_ChoppalbeTree_OJS OtherActor))
        (Utilities|IsValid _asbp_choppalbe_tree_ojs
          (:Is%20Valid
            (Class|BPIChoppable|Chop(Message) _asbp_choppalbe_tree_ojs 0.5)
            (Game|SpawnActorfromClass "/Game/00_OJS/tree/BP_ChoppingSpher_OJS.BP_ChoppingSpher_OJS_C" (Math|Transform|MakeTransform (Math|Vector|MakeVector (.x (Transformation|GetActorLocation _asbp_choppalbe_tree_ojs)) (.y (Transformation|GetActorLocation _asbp_choppalbe_tree_ojs)) (+ (.z (Transformation|GetActorLocation _asbp_choppalbe_tree_ojs)) 1.2e+02)) "0, 0, 0" "1.000000,1.000000,1.000000") "Undefined" "MultiplyWithRoot" 0 0)))))
    (:then_2
      (if (== (Utilities|GetClass OtherActor) "/Game/00_JWK/Blueprint/BP_Enemy/Boss/BP_Enemy_Boss.BP_Enemy_Boss_C")
        (bind _returnvalue (Actor|GetActorOfClass "/Game/00_JWK/Blueprint/BP_Enemy/Boss/BP_Enemy_Boss.BP_Enemy_Boss_C"))
        (Class|BossEnemy|BossTakeDamaged _returnvalue 1)))
    (:then_3
      (if (== (Utilities|GetClass OtherActor) "/Game/00_JWK/Blueprint/BP_Enemy/Goblin/BP_Enemy_Goblin.BP_Enemy_Goblin_C")
        (bind _returnvalue_2 (Actor|GetActorOfClass "/Game/00_JWK/Blueprint/BP_Enemy/Goblin/BP_Enemy_Goblin.BP_Enemy_Goblin_C"))
        (Class|GoblinEnemy|GoblinTakeDamaged _returnvalue_2 1)))))

(fn ConstructionScript)