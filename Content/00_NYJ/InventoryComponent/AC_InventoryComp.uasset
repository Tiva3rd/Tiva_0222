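; Inventory component that stores picked-up items as classes and shows them in an inventory widget.
; Show builds a five-column widget for the local player controller and hide removes it, both switching input mode and cursor unless the Controller check is set.
; Adding an item refreshes any valid widget.
; Spawn requests pass through client and server events to spawn the actor, ignoring collisions.
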(event Custom|Server%20Spawn%20Item
  (params (Class :type Actor%20Object%20Reference) (SpawnTransform :type Transform))
  ;[1 1 1] manage component로 해라?
  (Game|SpawnActorfromClass Class SpawnTransform "AlwaysSpawn" "MultiplyWithRoot" 0 0))

(event Custom|Client_SpawnItem
  (params (Class :type Actor%20Class%20Reference) (SpawnTransform :type Transform))
  ;[1 1 1] manage component로 해라?
  (CallFunction|ServerSpawnItem Class SpawnTransform))

(event EventFSpawnItem
  (params (ItemToSpawn :type BP%20Master%20Item%20Class%20Reference) (SpawnTransform :type Transform))
  ;[1 1 1] manage component로 해라?
  (CallFunction|ClientSpawnItem ItemToSpawn SpawnTransform))

(fn FShowInventroy
  (bind _returnvalue (Game|GetPlayerController 0))
  (if (Pawn|IsLocalController _returnvalue)
    (bind _returnvalue_2 (Game|ConstructObjectfromClass _returnvalue "/Game/00_NYJ/InventoryComponent/WBP_Inventory_NYJ.WBP_Inventory_NYJ_C"))
    (bind _output_get (Variables|Default|SetWBP_Inventory _returnvalue_2))
    (UserInterface|Viewport|AddtoViewport _output_get 0)
    (Default|FUpdate _returnvalue_2 (Variables|Default|GetInventory))
    (if (not (Variables|Default|GetController?))
      (Input|SetInputModeGameandUI (Game|GetPlayerController 0) (Variables|Default|GetWBP_Inventory) "LockInFullscreen" true false)
      (Variables|/Script/Engine.PlayerController|SetbShowMouseCursor (Game|GetPlayerController 0) true))))

(fn FHideInventory
  (Utilities|IsValid (Variables|Default|GetWBP_Inventory)
    (:Is%20Valid
      (Widget|RemovefromParent (Variables|Default|GetWBP_Inventory))
      (if (not (Variables|Default|GetController?))
        (Input|SetInputModeGameOnly (Game|GetPlayerController 0) false)
        (Variables|/Script/Engine.PlayerController|SetbShowMouseCursor (Game|GetPlayerController 0) false)))))

(fn FItemAddtoInentory
  (params (NewItem :type BP%20Master%20Item%20Object%20Reference%20%28by%20ref%29))
  (Utilities|Array|Add (Variables|Default|GetInventory) (Utilities|GetClass NewItem))
  (Utilities|IsValid (Variables|Default|GetWBP_Inventory)
    (:Is%20Valid
      (Default|FUpdate (Variables|Default|GetWBP_Inventory) (Variables|Default|GetInventory)))))