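; Wall-building component for BP_Archer: toggles a build mode that previews a wall and spawns BP_WallT on install.
; Each tick in build mode, a camera line trace moves a collision-free preview mesh, created once through a DoOnce that resets when the mode ends.
; Holding Q or E rotates the preview in fixed yaw steps.
; Toggle, install and rotation pass through C2S-to-S2M event pairs, named for client-to-server-to-multicast relay.
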(event Custom|PreviewLoop
  (bind _camera (Variables|Default|GetCamera))
  (bind _returnvalue (Transformation|GetWorldTransform _camera))
  ;[1 0.6224 0.7762] Custom event 모음
  (bind (_outhit _returnvalue_2) (Collision|LineTraceByChannel (.location _returnvalue) (+ (.location _returnvalue) (* (Math|Vector|GetForwardVector (.rotation _returnvalue)) 1e+03)) "TraceTypeQuery1" false 0 "None"))
  (if _returnvalue_2
    (Utilities|FlowControl|Sequence
      (:then_0
        (Utilities|FlowControl|DoOnce false
          (:Completed
            (bind _returnvalue_3 (Game|AddComponentbyClass (Variables|Default|GetplayerBp3) "/Script/Engine.StaticMeshComponent" false (Variables|Default|GetbuildPreviewTransform)))
            (bind _output_get (Variables|Default|SetPreview%20Mesh _returnvalue_3))
            (Components|StaticMesh|SetStaticMesh _output_get "/Game/00_OJS/wall/MAKEWALLT.MAKEWALLT")
            (Rendering|Material|SetMaterial (Variables|Default|GetPreview%20Mesh) 0 "/Game/00_OJS/build/M_buildPreview.M_buildPreview")
            (Collision|SetCollisionEnabled (Variables|Default|GetPreview%20Mesh) "NoCollision"))))
      (:then_1
        (bind _output_get_2 (Variables|Default|SetbuildPreviewTransform (Math|Transform|MakeTransform (.Location (Collision|BreakHitResult _outhit)) (Variables|Default|GetbuildPreviewRotation) "1.000000,1.000000,1.000000")))
        (Transformation|SetWorldTransform (Variables|Default|GetPreview%20Mesh) _output_get_2 false false)))))

(event Custom|reset%20build%20mode
  ;[1 0.6224 0.7762] Custom event 모음
  (Utilities|FlowControl|DoOnce false) ; enters at Reset
)

(event Custom|PressQ_S2M
  ;[1 1 1] 반시계 회전
  (Variables|Default|SetbuildPreviewRotation (Math|Rotator|CombineRotators (.rotation (Variables|Default|GetbuildPreviewTransform)) "0.000000,-5.000000,0.000000")))

(event Custom|stopbuildMode
  ;[1 1 1] 프리뷰
  (Variables|Default|SetisBuildMode false)
  (bind _preview_mesh (Variables|Default|GetPreview%20Mesh)
    (:then
      (Components|StaticMesh|SetStaticMesh _preview_mesh 0)
      (Variables|Default|SetPreview%20Mesh 0)
      (CallFunction|ResetBuildMode))
    (:else)))

(event Custom|Preview_C2S
  (CallFunction|PreviewS2M))

(event Custom|Install_C2S
  (CallFunction|InstallS2M))

(event Custom|PressQ_C2S
  ;[1 1 1] 반시계 회전
  (CallFunction|PressQS2M))

(event Custom|PressE_C2S
  ;[1 1 1] 시계 회전
  (CallFunction|PressES2M))

(event Custom|PressE_S2M
  ;[1 1 1] 시계 회전
  (Variables|Default|SetbuildPreviewRotation (Math|Rotator|CombineRotators (.rotation (Variables|Default|GetbuildPreviewTransform)) "0.000000,5.000000,0.000000")))

(event Custom|Preview_S2M
  ;[1 1 1] 프리뷰
  (if (not (Variables|Default|GetisBuildMode))
    (Variables|Default|SetisBuildMode true)
    (else
      (Variables|Default|SetisBuildMode false)
      (bind _preview_mesh (Variables|Default|GetPreview%20Mesh)
        (:then
          (Components|StaticMesh|SetStaticMesh _preview_mesh 0)
          (Variables|Default|SetPreview%20Mesh 0)
          (CallFunction|ResetBuildMode))
        (:else)))))

(event Custom|Install_S2M
  ;[1 1 1] 설치
  (if (Variables|Default|GetisBuildMode)
    (Game|SpawnActorfromClass "/Game/00_OJS/wall/BP_WallT.BP_WallT_C" (Variables|Default|GetbuildPreviewTransform) "Undefined" "MultiplyWithRoot" 0 0)
    (CallFunction|StopbuildMode)))

(event EventBeginPlay
  (bind _asbp_archer (Utilities|Casting|CastToBP_Archer (Components|GetOwner)))
  (Variables|Default|SetplayerBp3 _asbp_archer)
  (Variables|Default|SetCamera (Variables|/Script/Tiva.TivaCharacter|GetFollowCamera _asbp_archer)))

(event EventTick
  (params (DeltaSeconds :type Float%20%28single-precision%29))
  (if (Variables|Default|GetisBuildMode)
    (CallFunction|PreviewLoop)
    (if (Variables|Default|GetReverse)
      (CallFunction|PressQC2S)
      (elif (Variables|Default|GetForwad)
        (CallFunction|PressEC2S)))))

(event Input|KeyboardEvents|E
  (params (Key :type Key%20Structure :default "None"))
  ;[1 1 1] 시계 회전
  (:Pressed
    (Variables|Default|SetForwad true))
  (:Released
    (Variables|Default|SetForwad false)))

(event Input|KeyboardEvents|Q
  (params (Key :type Key%20Structure :default "None"))
  ;[1 1 1] 반시계 회전
  (:Pressed
    (Variables|Default|SetReverse true))
  (:Released
    (Variables|Default|SetReverse false)))