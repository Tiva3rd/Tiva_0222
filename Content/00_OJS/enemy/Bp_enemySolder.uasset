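; Soldier character that, despite its enemy name, acts as a quest-giving NPC, briefly showing an interaction prompt when BP_Archer touches its capsule.
; Custom events drive ACQuest and the message, mission and mini-quest widgets, ending with a request for ore and wood.
; The first mission event enables InteractColl, which reports overlapping BP_MasterItem actors to ACQuest as pickups.
; The follow-and-melee chase event has no live caller here.
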(event OnSeePawn(PawnSensing)
  (params (Pawn :type Pawn%20Object%20Reference)))

(event OnComponentBeginOverlap(InteractColl)
  (params (OverlappedComponent :type Primitive%20Component%20Object%20Reference) (OtherActor :type Actor%20Object%20Reference) (OtherComp :type Primitive%20Component%20Object%20Reference) (OtherBodyIndex :type Integer) (bFromSweep :type Boolean) (SweepResult :type Hit%20Result%20Structure%20%28by%20ref%29))
  (if (== (Utilities|GetClass OtherActor) "/Game/00_NYJ/InventoryComponent/Item/BP_MasterItem.BP_MasterItem_C")
    (Development|PrintString "Hello")
    (Default|FItemPickup (Variables|Default|GetAC_Quest))))

(event OnComponentBeginOverlap(CapsuleComponent)
  (params (OverlappedComponent :type Primitive%20Component%20Object%20Reference) (OtherActor :type Actor%20Object%20Reference) (OtherComp :type Primitive%20Component%20Object%20Reference) (OtherBodyIndex :type Integer) (bFromSweep :type Boolean) (SweepResult :type Hit%20Result%20Structure%20%28by%20ref%29))
  (if (== (Utilities|GetClass OtherActor) "/Game/00_NYJ/Character/BP_Archer.BP_Archer_C")
    (Widget|SetVisibility (Variables|Default|GetInteractionF) "Visible")
    (Utilities|FlowControl|Delay 1.0)
    (Widget|SetVisibility (Variables|Default|GetInteractionF) "Hidden")))

(event Custom|FollowPlayer
  (Utilities|FlowControl|DoOnce false :!label _label
    (:Completed
      (AI|AIMoveTo self "0, 0, 0" (Game|GetPlayerCharacter 0) 5e+01 false
        (:OnSuccess
          (Components|Animation|PlayAnimation (Variables|Character|GetMesh) "/Game/00_OJS/TREE2/Standing_Melee_Attack_Downward__1_.Standing_Melee_Attack_Downward__1_" false)
          (goto _label Reset))))))

(event Custom|Show%20MessageUI_NpcMeet
  (Default|FSetStateQuest (Variables|Default|GetAC_Quest) "NewEnumerator0")
  (bind _returnvalue (UserInterface|CreateWidget "/Game/00_OJS/enemy/WBP_TEXT.WBP_TEXT_C"))
  (UserInterface|Viewport|AddtoViewport _returnvalue 0)
  (Utilities|FlowControl|Delay 5.0)
  (Widget|RemovefromParent _returnvalue)
  (bind _returnvalue_2 (UserInterface|CreateWidget "/Game/00_NYJ/NPC/WBP_MiniQuest.WBP_MiniQuest_C"))
  (Variables|Default|SetCurrentMiniUI _returnvalue_2)
  (UserInterface|Viewport|AddtoViewport _returnvalue_2 0))

(event Custom|Show_UI_2nd
  (bind _currentminiui (Variables|Default|GetCurrentMiniUI))
  (Development|PrintString "2nd")
  (Widget|SetVisibility _currentminiui "Visible")
  (Variables|/Script/UMG.TextBlock|SetText (Variables|/Game/00_NYJ/NPC/WBP_MiniQuest.WBP_MiniQuest_C|GetQuestText _currentminiui) "광석 3개와 나무3개를 가져오시오."))

(event Custom|Show_UI_1st
  (Utilities|FlowControl|Sequence
    (:then_0
      (Widget|SetVisibility (Variables|Default|GetCurrentMiniUI) "Hidden")
      (Development|PrintString "아이템  내놔라")
      (Default|FItemPickup (Variables|Default|GetAC_Quest))
      ;[1 1 1] 아이템을 내놓으라는 UI
      (bind _returnvalue (UserInterface|CreateWidget "/Game/00_OJS/enemy/WBP_Mission1.WBP_Mission1_C"))
      (UserInterface|Viewport|AddtoViewport _returnvalue 0)
      (Utilities|FlowControl|Delay 5.0)
      (Widget|RemovefromParent _returnvalue))
    (:then_1
      (Development|PrintString "Collision Enabled")
      (Collision|SetCollisionEnabled (Variables|Default|GetInteractColl) "QueryAndPhysics"))))

(event EventBeginPlay
  (|CallParentFunction)
  (bind _returnvalue (UserInterface|CreateWidget "/Game/00_NYJ/InventoryComponent/WBP/WBP_InteractionNPC.WBP_InteractionNPC_C"))
  (bind _output_get (Variables|Default|SetInteractionF _returnvalue))
  (UserInterface|Viewport|AddtoViewport _returnvalue 0)
  (Widget|SetVisibility _output_get "Hidden")
  (Collision|SetCollisionEnabled (Variables|Default|GetInteractColl) "NoCollision"))

(event Collision|EventActorBeginOverlap
  (params (OtherActor :type Actor%20Object%20Reference)))

(event EventTick
  (params (DeltaSeconds :type Float%20%28single-precision%29))
  (|CallParentFunction DeltaSeconds) ; This node is disabled and will not be called.\nDrag off pins to build functionality.
)

(fn ConstructionScript
  (|CallParentFunction))