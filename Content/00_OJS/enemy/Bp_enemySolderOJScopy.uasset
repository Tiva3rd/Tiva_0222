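; Enemy soldier pawn that moves toward the player when its pawn sensing sees a pawn.
; Sight triggers a DoOnce-gated AI MoveTo that targets the player controller rather than its pawn.
; On arrival it briefly raises the ChopAndMiningBP flag, then resets the gate; a failed move leaves it closed.
; Code creating a hidden NPC interaction widget is present but never runs.
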(event OnSeePawn(PawnSensing)
  (params (Pawn :type Pawn%20Object%20Reference))
  (CallFunction|FollowPlayer))

(event Custom|FollowPlayer
  (bind _self self)
  (Utilities|FlowControl|DoOnce false :!label _label
    (:Completed
      (AI|AIMoveTo _self "0, 0, 0" (Game|GetPlayerController 0) 1e+02 false
        (:OnSuccess
          (Variables|Default|SetChopAndMiningBP _self true)
          (Utilities|FlowControl|Delay 1.5)
          (Variables|Default|SetChopAndMiningBP false)
          (goto _label Reset))))))

(event EventBeginPlay
  (|CallParentFunction))

(event Collision|EventActorBeginOverlap
  (params (OtherActor :type Actor%20Object%20Reference)))

(event EventTick
  (params (DeltaSeconds :type Float%20%28single-precision%29))
  (|CallParentFunction DeltaSeconds) ; This node is disabled and will not be called.\nDrag off pins to build functionality.
)

(fn ConstructionScript
  (|CallParentFunction))