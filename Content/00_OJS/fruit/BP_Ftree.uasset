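; BP_Ftree is a fruit tree that grows apples at its arrow components and drops them when a player character hits it.
; A looping timer randomly fills empty slots with small static mesh apples.
; A hit swaps those meshes for short-lived Apple actors, then after a delay spawns a BP_TreeMaterial item near the tree.
; That item's stack is the total slot count, and spawning it clears the slot array, ending regrowth.
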(event OnComponentHit(StaticMesh)
  (params (HitComponent :type Primitive%20Component%20Object%20Reference) (OtherActor :type Actor%20Object%20Reference) (OtherComp :type Primitive%20Component%20Object%20Reference) (NormalImpulse :type Vector :default "0, 0, 0") (Hit :type Hit%20Result%20Structure%20%28by%20ref%29))
  (Utilities|FlowControl|Sequence
    (:then_0
      (Utilities|Casting|CastToBP_MyCharacter_tivaOJS OtherActor))
    (:then_1
      (Utilities|Casting|CastToBP2_MyCharacter2_tiva2OJS2 OtherActor))
    (:then_2
      (Utilities|Casting|CastToBP_Archer OtherActor)))
  (for (_array_element _array_index) (Variables|Default|GetAppleSpawned)
    (if _array_element
      (Utilities|Array|SetArrayElem (Variables|Default|GetAppleSpawned) _array_index false)
      (bind _returnvalue (Game|SpawnActorfromClass "/Game/00_OJS/fruit/Apple.Apple_C" (Math|Transform|MakeTransform (Transformation|GetWorldLocation (Utilities|Array|Get(acopy) (Variables|Default|GetAppleLocation) _array_index)) "0, 0, 0" "1.000000,1.000000,1.000000") "Undefined" "MultiplyWithRoot" 0 0))
      (Components|DestroyComponent (Components|GetChildComponent (Utilities|Array|Get(acopy) (Variables|Default|GetAppleLocation) _array_index) 0))
      (Utilities|FlowControl|Sequence
        (:then_0
          (Utilities|FlowControl|Delay 4.0)
          (Development|PrintString "c2s")
          (CallFunction|SpawnItemC2S))
        (:then_1
          (Utilities|FlowControl|Delay 2.0)
          (Actor|DestroyActor _returnvalue))))))

(event Custom|SpawnApples
  (for (_array_element _array_index) (Variables|Default|GetAppleSpawned)
    (if (not _array_element)
      (if (>= (Math|Random|RandomFloatinRange 0.0 1e+02) 5e+01)
        (Utilities|Array|SetArrayElem (Variables|Default|GetAppleSpawned) _array_index true)
        (bind _returnvalue (AddComponent|AddStaticMeshComponent false (Math|Transform|MakeTransform "0, 0, 0" "0, 0, 0" "0.150000,0.150000,0.150000")))
        (Transformation|AttachComponentToComponent _returnvalue (Utilities|Array|Get(acopy) (Variables|Default|GetAppleLocation) _array_index) "None" "SnapToTarget" "SnapToTarget" "KeepRelative" true)))))

(event Custom|SpawnItemC2S
  (bind _output_get (Variables|Default|SetNewItemSpawn (Math|Conversions|ToTransform(Vector) (+ (+ (Transformation|GetActorLocation) (* (Math|Vector|Normalize (Math|Vector|GetUpVector (Transformation|GetActorRotation))) (Variables|Default|GetItem%20Drop%20Distance))) (Math|Vector|MakeVector (Math|Random|RandomFloatinRange -75.0 75.0) (Math|Random|RandomFloatinRange -75.0 75.0) 0.0)))))
  (CallFunction|SpawnItemS2M _output_get (Utilities|Array|Length (Variables|Default|GetAppleSpawned))))

(event Custom|SpawnItemS2M
  (params (Spawn :type Transform) (AppleCount :type Integer))
  (Game|SpawnActorfromClass "/Game/00_NYJ/InventoryComponent/Item/BP_TreeMaterial.BP_TreeMaterial_C" Spawn "Undefined" "MultiplyWithRoot" 0 false false AppleCount 0)
  (Development|PrintString "spawn s2m")
  (Utilities|Array|Clear (Variables|Default|GetAppleSpawned)))

(event EventBeginPlay
  (bind _output_get (Variables|Default|SetAppleLocation (Actor|GetComponentsByClass "/Script/Engine.ArrowComponent")))
  (Utilities|Array|Resize (Variables|Default|GetAppleSpawned) (Utilities|Array|Length _output_get))
  (Utilities|Time|SetTimerbyEvent (delegate Custom|SpawnApples) 5.0 true))

(fn ConstructionScript)