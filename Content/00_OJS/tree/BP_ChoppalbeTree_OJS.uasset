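; Choppable tree actor that gets felled by repeated hits and drops a BP_MasterItem pickup.
; Each Chop adds hand damage to Chopvalue, which drives the Hardness parameter on a dynamic trunk material.
; Once Chopvalue reaches its threshold, a procedural copy made at construction replaces the static mesh, gets sliced with a wood cap, and enables physics.
; MoveComponentTo then animates it, the item spawns nearby, and the tree sinks and is destroyed.
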(event EventBeginPlay
  (bind _returnvalue (Rendering|Material|CreateDynamicMaterialInstance "/Game/00_OJS/tree/M_tree_Inst.M_tree_Inst" "None" "None" :!class /Script/Engine.KismetMaterialLibrary))
  (bind _output_get (Variables|Default|SetMaterial2 _returnvalue))
  (Rendering|Material|SetMaterial (Variables|Default|GetStaticMesh) 0 _output_get)
  (Collision|SetCollisionEnabled (Variables|Default|GetProceduralMesh) "QueryAndPhysics"))

(event Collision|EventActorBeginOverlap
  (params (OtherActor :type Actor%20Object%20Reference)))

(event EventChop
  (params (DamageHand :type Float%20%28double-precision%29))
  (bind _self self)
  (bind _proceduralmesh (Variables|Default|GetProceduralMesh))
  (bind _staticmesh (Variables|Default|GetStaticMesh))
  (bind _returnvalue (Transformation|GetWorldLocation _staticmesh))
  (if (>= (Variables|Default|Getchopvalue) 0.4)
    (Rendering|SetVisibility (Variables|Default|GetStaticMesh) false false)
    (Rendering|SetVisibility _proceduralmesh true false)
    (Class|KismetProceduralMeshLibrary|SliceProceduralMesh _proceduralmesh (Math|Vector|MakeVector (.x _returnvalue) (.y _returnvalue) (+ (.z _returnvalue) 1.1e+02)) (Math|Vector|MakeVector 0.2 0.2 1.0) true "UseLastSectionForCap" "/Game/Megascans/Surfaces/Wood_qklp2op0/MI_Wood_qklp2op0_2K.MI_Wood_qklp2op0_2K")
    (Physics|SetSimulatePhysics _proceduralmesh true)
    (Physics|SetEnableGravity _proceduralmesh true)
    (Rendering|Material|SetMaterial (Variables|Default|GetProceduralMesh) 0 "/Game/Megascans/3D_Assets/Blackened_Tree_Trunk_vclpbigga/MI_Blackened_Tree_Trunk_vclpbigga_2K.MI_Blackened_Tree_Trunk_vclpbigga_2K")
    (Components|MoveComponentTo (Variables|Default|GetProceduralMesh) "0.000000,0.000000,20.000000" "90.000000,0.000000,0.000000" false false 2.0 false)
    (Utilities|FlowControl|Sequence
      (:then_0
        (Components|MoveComponentTo (Variables|Default|GetProceduralMesh) "0.000000,0.000000,-100.000000" "90.000000,0.000000,0.000000" false false 3.0 false)
        (Components|DestroyComponent (Variables|Default|GetProceduralMesh))
        (Collision|SetActorEnableCollision false)
        (Utilities|FlowControl|Delay 3.0)
        (Actor|DestroyActor))
      (:then_1
        (Game|SpawnActorfromClass "/Game/00_NYJ/InventoryComponent/BP_MasterItem.BP_MasterItem_C" (Math|Conversions|ToTransform(Vector) (+ (+ (Transformation|GetActorLocation _self) (* (Math|Vector|Normalize (Math|Vector|GetUpVector (Transformation|GetActorRotation _self))) (Variables|Default|GetItem%20Drop%20Distance))) (Math|Vector|MakeVector (Math|Random|RandomFloatinRange -75.0 75.0) (Math|Random|RandomFloatinRange -75.0 75.0) 0.0))) "AlwaysSpawn" "MultiplyWithRoot" 0 true false 0)))
    (else
      (bind _output_get (Variables|Default|Setchopvalue (+ (Variables|Default|Getchopvalue) DamageHand)))
      (Rendering|Material|SetScalarParameterValue (Variables|Default|GetMaterial2) "Hardness" _output_get :!class /Script/Engine.MaterialInstanceDynamic))))

(fn ConstructionScript
  (Class|KismetProceduralMeshLibrary|CopyProceduralMeshfromStaticMeshComponent (Variables|Default|GetStaticMesh) 0 (Variables|Default|GetProceduralMesh) false))

(fn IsChoppable?
  (return true))